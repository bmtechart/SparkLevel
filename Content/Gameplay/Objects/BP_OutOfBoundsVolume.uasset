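; Out-of-bounds trigger volume that resets the player Spark character to a safe position when it falls in.
; A box overlap calls the character's reset through a DoOnce gate, which re-arms when the character's reset-complete callback fires.
; The construction script toggles an optional debug plane and keeps it aligned to the top of the box.
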(event `self.OutOfBoundsCollision.OnComponentBeginOverlap`
  (params (OverlappedComponent :type "PrimitiveComponent Object Reference") (OtherActor :type "Actor Object Reference") (OtherComp :type "PrimitiveComponent Object Reference") (OtherBodyIndex :type Integer) (bFromSweep :type Boolean) (SweepResult :type "HitResult Structure (by ref)"))
  ;[1 1 1] When the player falls into the volume, reset them
  (bind _asbp_spark_character_player (cast `/Game/Gameplay/Characters/Player/BP_SparkCharacter_Player` OtherActor))
  (`/Engine/EditorBlueprintResources/StandardMacros.DoOnce` false :!label _label
    (:`Completed`
      (`/Game/Gameplay/Characters/Player/BP_SparkCharacter_Player.ResetToSafePosition` _asbp_spark_character_player)
      (add `/Game/Gameplay/Characters/Player/BP_SparkCharacter_Player.OnResetToSafeLocationComplete` _asbp_spark_character_player (delegate `OnResetToSafeLocationComplete_Event_0`)))))

(event `OnResetToSafeLocationComplete_Event_0`
  ;[1 1 1] When the player falls into the volume, reset them
  (goto _label :!via `Reset`))

(fn `UserConstructionScript`
  (bind (_returnvalue_x _returnvalue_y _returnvalue_z) (`KismetMathLibrary.BreakVector` (`self.K2_GetActorLocation`)))
  (bind (_returnvalue_x_2 _returnvalue_y_2 _returnvalue_z_2) (`KismetMathLibrary.BreakVector` (`BoxComponent.GetScaledBoxExtent` (`self.OutOfBoundsCollision`))))
  ;[1 1 1] Whether or not to draw the plane
  (`SceneComponent.SetVisibility` (`self.DebugPlane`) (`self.DrawDebugMaterial`) false)
  ;[1 1 1] Make sure the plane is always as the very utmost top of the box
  (`SceneComponent.K2_SetWorldLocation` (`self.DebugPlane`) (`KismetMathLibrary.MakeVector` _returnvalue_x _returnvalue_y (+ _returnvalue_z_2 _returnvalue_z)) false false))