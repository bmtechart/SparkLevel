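; Tornado actor that catches the Stormwrak player on overlap and carries them along a spline lined with collectible-style gems.
; The construction script builds spline meshes along the path with a dynamic twister material.
; Gems spawn at BeginPlay unless already spawned from the editor.
; One timeline snaps the player to the nearest spline point, then another, rate-scaled for constant speed, moves them to the end and re-enables input.
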(event `Clear Gems`
  (for _array_element (`self.Gems`)
    (`self.K2_DestroyActor` _array_element))
  (`KismetArrayLibrary.Array_Clear` (`self.Gems`))
  (set `self.GemsSpawnedFromEditor?` false))

(event `Spawn Gems Along Spline`
  (if (> (`KismetArrayLibrary.Array_Length` (`self.Gems`)) 0)
    (`self.Clear Gems`))
  ;[1 1 1] Spawn gems along spline
  (bind _outtransforms (`/Game/Users/BrianMurphy/Blueprints/BPFL_SplineFunctions.Transforms Along Spline` (`self.spliney_splineboy`) "/Script/Engine.Actor" (`self.Gem Density`) (`self.Gem Start Key`) (`self.Gem End Key`) false 0 false "World"))
  (for (_array_element _array_index) _outtransforms
    (bind _returnvalue (`|SpawnActorFromClass` "/Game/Gameplay/Objects/BP_Gem.BP_Gem_C" (`KismetMathLibrary.MakeTransform` (.location _array_element) (.rotation _array_element) (* (.scale _array_element) (`self.Gem Scale`))) "Undefined" "OverrideRootScale" null "NewEnumerator4" (struct) 120.0 null))
    (`KismetArrayLibrary.Array_Set` (`self.Gems`) _array_index _returnvalue true))
  (set `self.GemsSpawnedFromEditor?` true))

(event `self.ReceiveBeginPlay`
  (`|ExecutionSequence`
    (:`then_0`
      (if (not (`self.GemsSpawnedFromEditor?`))
        (`self.Spawn Gems Along Spline`)))
    (:`then_1`
      ;[1 1 1] Set play rate
      (`TimelineComponent.SetPlayRate` (`self.SplineLengthTimeline`) (/ 1.0 (/ (`SplineComponent.GetSplineLength` (`self.spliney_splineboy`)) (`self.SplineMovementSpeed`)))))))

(event `self.ReceiveActorBeginOverlap`
  (params (OtherActor :type "Actor Object Reference"))
  (bind _returnvalue (`self.K2_GetActorLocation` (`self.Spark`)))
  (bind _returnvalue_2 (`SplineComponent.FindInputKeyClosestToWorldLocation` (`self.spliney_splineboy`) _returnvalue))
  ;[0 0.09028 1 1 60] Player Enters Twister
  (bind _asbp_spark_character_player_stormwrak (cast `/Game/Users/BrianMurphy/Blueprints/BP_SparkCharacter_Player_Stormwrak` OtherActor))
  (`/Engine/EditorBlueprintResources/StandardMacros.DoOnce` false :!label _label
    (:`Completed`
      (set `self.Spark` _asbp_spark_character_player_stormwrak)
      (if (`self.enabled`)
        (`/Engine/EditorBlueprintResources/StandardMacros.IsValid` (`self.Spark`)
          (:`Is Valid`
            (`|ExecutionSequence`
              (:`then_0`
                ;;[1 1 1] If the player has left a tornado and is still decelerating, invalidate that timer handle
                (if (`KismetSystemLibrary.K2_IsValidTimerHandle` (`self.BlendVelocityTimerHandle`))
                  (`KismetSystemLibrary.K2_ClearAndInvalidateTimerHandle` (`self.BlendVelocityTimerHandle`))))
              (:`then_1`
                ;;[1 1 1] Get Closest Input Key On Spline
                (set `self.InitialInputKey` _returnvalue_2)
                (`self.MoveToSpline` _returnvalue_2 _returnvalue)))))))))

(event `Reset`
  ;[0 0.09028 1 1 60] Player Enters Twister
  (goto _label :!via `Reset`))

(event `MoveToSpline`
  (params (InputKey :type "Float (double-precision)") (InitialPosition :type "Vector Structure"))
  (bind _spliney_splineboy (`self.spliney_splineboy`))
  ;[1 1 1 1 50] Smooth Snap to Spline
  (`/Engine/EditorBlueprintResources/StandardMacros.IsValid` (`self.Spark`)
    (:`Is Valid`
      (bind (_direction _splinekey) (`Timeline|MoveToSplineTimeline` :!via `PlayFromStart`)
        (:`Update`
          (`self.K2_SetActorLocation` (`self.Spark`) (`KismetMathLibrary.VLerp` InitialPosition (`SplineComponent.GetLocationAtSplineInputKey` _spliney_splineboy InputKey "World") _splinekey) false false))
        (:`Finished`
          (`TimelineComponent.SetNewTime` (`self.SplineLengthTimeline`) (/ (`SplineComponent.GetDistanceAlongSplineAtSplineInputKey` _spliney_splineboy InputKey) (`SplineComponent.GetSplineLength` _spliney_splineboy)))
          (`self.MoveUpSpline`))))))

(event `MoveUpSpline`
  ;[1 1 1 1 50] Move Along Length of Spline
  (`/Engine/EditorBlueprintResources/StandardMacros.IsValid` (`self.Spark`)
    (:`Is Valid`
      (bind (_direction _splinekey) (`Timeline|SplineLengthTimeline`)
        (:`Update`
          ;;[1 1 1] Update Player Position
          (`self.K2_SetActorLocation` (`self.Spark`) (`SplineComponent.GetLocationAtDistanceAlongSpline` (`self.spliney_splineboy`) (`KismetMathLibrary.Lerp` 0.0 (`SplineComponent.GetSplineLength` (`self.spliney_splineboy`)) _splinekey) "World") false false))
        (:`Finished`
          (`/Game/Gameplay/Characters/BP_SparkCharacter.EnableCharacterControllerInput` (`self.Spark`))
          (`self.Reset`))))))

(fn `Smooth Move to Spline`
  (params (Spline :type "SplineComponent Object Reference") (SplineInputKey :type "Float (double-precision)") (ActorToMove :type "Actor Object Reference"))
  (returns (TargetPositionReached :type Boolean))
  (bind _returnvalue (`SplineComponent.GetLocationAtSplineInputKey` Spline SplineInputKey "World"))
  (bind _returnvalue_2 (`KismetMathLibrary.VInterpTo` (`self.K2_GetActorLocation` ActorToMove) _returnvalue (`GameplayStatics.GetWorldDeltaSeconds`)))
  (`self.K2_SetActorLocation` ActorToMove _returnvalue_2 true false)
  (return (== _returnvalue _returnvalue_2)))

(fn `Smooth Move Up Spline`
  (params (Spline :type "SplineComponent Object Reference") (`Actor To Move` :type "Actor Object Reference") (`Move Rate` :type "Float (double-precision)"))
  (returns (`Spline Top Reached` :type Boolean))
  (return false))

(fn `UserConstructionScript`
  (bind _width_multiplier (`self.Width Multiplier`))
  (bind _spliney_splineboy (`self.spliney_splineboy`))
  (`|ExecutionSequence`
    (:`then_0`
      ;[1 1 1] Clear existing meshes
      (for _array_element (`self.SplineMeshes`)
        (`ActorComponent.K2_DestroyComponent` _array_element))
      (`KismetArrayLibrary.Array_Clear` (`self.SplineMeshes`)))
    (:`then_1`
      ;[1 1 1] Create material
      (bind _returnvalue (`KismetMaterialLibrary.CreateDynamicMaterialInstance` "/Game/Users/BrianMurphy/Materials/M_Twister.M_Twister"))
      (bind _output_get (set `self.DynamicMaterialInstance` _returnvalue))
      ;[1 1 1] Set material instance parameters
      (`MaterialInstanceDynamic.SetVectorParameterValue` _output_get "InnerColour" (`self.InnerColour`))
      (`MaterialInstanceDynamic.SetVectorParameterValue` (`self.DynamicMaterialInstance`) "OuterColour" (`self.OuterColour`))
      (`MaterialInstanceDynamic.SetScalarParameterValue` (`self.DynamicMaterialInstance`) "MinDisplacement" (`self.MinDisplacement`))
      (`MaterialInstanceDynamic.SetScalarParameterValue` (`self.DynamicMaterialInstance`) "MaxDisplacement" (`self.MaxDisplacement`)))
    (:`then_2`
      ;[1 1 1] Generate pSpline Meshes
      (for _index (range (+ (`KismetMathLibrary.FTrunc` (/ (`SplineComponent.GetSplineLength` (`self.spliney_splineboy`)) (`self.SectionLength`))) 1))
        (bind _returnvalue_2 (`AddComponent|NODE_AddSplineMeshComponent-1` :`RelativeTransform` (`KismetMathLibrary.MakeTransform` (0.0 0.0 0.0) (struct) (`KismetMathLibrary.MakeVector` _width_multiplier _width_multiplier 1.0))))
        (`SplineMeshComponent.SetForwardAxis` _returnvalue_2 "Z" true)
        (`PrimitiveComponent.SetMaterial` _returnvalue_2 0 (`self.DynamicMaterialInstance`))
        (`KismetArrayLibrary.Array_Set` (`self.SplineMeshes`) _index _returnvalue_2 true)
        (`SceneComponent.K2_AttachToComponent` _returnvalue_2 (`self.spliney_splineboy`) "None" "KeepRelative" "KeepRelative" "KeepRelative" false)
        (bind _returnvalue_3 (* _index (`self.SectionLength`)))
        (bind _returnvalue_4 (* (+ _index 1) (`self.SectionLength`)))
        (`SplineMeshComponent.SetStartAndEnd` _returnvalue_2 (`SplineComponent.GetLocationAtDistanceAlongSpline` _spliney_splineboy _returnvalue_3 "Local") (`SplineComponent.GetTangentAtDistanceAlongSpline` _spliney_splineboy _returnvalue_3 "Local") (`SplineComponent.GetLocationAtDistanceAlongSpline` _spliney_splineboy _returnvalue_4 "Local") (`SplineComponent.GetTangentAtDistanceAlongSpline` _spliney_splineboy _returnvalue_4 "Local") true)))))