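; Enemy spawner actor that spawns one orc AI character of a requested type at its own transform.
; SpawnEnemy plays a smoke effect and sound, then switches on EnemyType to spawn an Archer, Warrior, Brute (Grunt) or Mage (Shaman).
; All but the Archer get CanLoseTarget disabled; the TargetingPlayer input is unused.
; It stores only the latest spawn, which KillSpawnedActor destroys if still valid.
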(event `SpawnEnemy`
  (params (TargetingPlayer :type Boolean) (EnemyType :type "/Game/Users/BrianMurphy/Blueprints/EEnemyType Enum" :default "NewEnumerator0"))
  (bind _returnvalue (`self.GetTransform`))
  (`NiagaraFunctionLibrary.SpawnSystemAtLocation` "/Game/Characters/Orc/FX/FX_OrcDeathSmoke_System.FX_OrcDeathSmoke_System")
  (`GameplayStatics.PlaySoundAtLocation` "/Game/Users/BrianMurphy/Audio/Ice_Spell_Ice_Spell_Buff_Positive_02.Ice_Spell_Ice_Spell_Buff_Positive_02" (`self.K2_GetActorLocation`) (struct) 1.0 1.0 0.0 null null null)
  (switch `/Game/Users/BrianMurphy/Blueprints/EEnemyType` EnemyType
    (:`NewEnumerator0`
      (bind _returnvalue_2 (`|SpawnActorFromClass` :`Class` "/Game/Gameplay/Characters/AI/Orcs/BP_SparkCharacter_AI_OrcArcher.BP_SparkCharacter_AI_OrcArcher_C" :`SpawnTransform` _returnvalue :`CollisionHandlingOverride` "Undefined" :`TransformScaleMethod` "OverrideRootScale" :`Instigator` null))
      (set `self.SpawnedActor` _returnvalue_2))
    (:`NewEnumerator1`
      (bind _returnvalue_3 (`|SpawnActorFromClass` :`Class` "/Game/Gameplay/Characters/AI/Orcs/BP_SparkCharacter_AI_OrcWarrior.BP_SparkCharacter_AI_OrcWarrior_C" :`SpawnTransform` _returnvalue :`CollisionHandlingOverride` "Undefined" :`TransformScaleMethod` "OverrideRootScale" :`Instigator` null))
      (set `self.SpawnedActor` _returnvalue_3)
      (set `/Game/Gameplay/Characters/AI/BP_SparkCharacter_AI.CanLoseTarget` false _returnvalue_3))
    (:`NewEnumerator2`
      (bind _returnvalue_4 (`|SpawnActorFromClass` :`Class` "/Game/Gameplay/Characters/AI/Orcs/BP_SparkCharacter_AI_OrcGrunt.BP_SparkCharacter_AI_OrcGrunt_C" :`SpawnTransform` _returnvalue :`CollisionHandlingOverride` "Undefined" :`TransformScaleMethod` "OverrideRootScale" :`Instigator` null))
      (set `self.SpawnedActor` _returnvalue_4)
      (set `/Game/Gameplay/Characters/AI/BP_SparkCharacter_AI.CanLoseTarget` false _returnvalue_4))
    (:`NewEnumerator3`
      (bind _returnvalue_5 (`|SpawnActorFromClass` :`Class` "/Game/Gameplay/Characters/AI/Orcs/BP_SparkCharacter_AI_OrcShaman.BP_SparkCharacter_AI_OrcShaman_C" :`SpawnTransform` _returnvalue :`CollisionHandlingOverride` "Undefined" :`TransformScaleMethod` "OverrideRootScale" :`Instigator` null))
      (set `self.SpawnedActor` _returnvalue_5)
      (set `/Game/Gameplay/Characters/AI/BP_SparkCharacter_AI.CanLoseTarget` false _returnvalue_5))))

(event `KillSpawnedActor`
  (`/Engine/EditorBlueprintResources/StandardMacros.IsValid` (`self.SpawnedActor`)
    (:`Is Valid`
      (`self.K2_DestroyActor` (`self.SpawnedActor`)))))

(fn `UserConstructionScript`)