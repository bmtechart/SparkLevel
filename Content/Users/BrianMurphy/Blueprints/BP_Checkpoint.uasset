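; BP_Checkpoint is a checkpoint actor that records a respawn point when the player enters its trigger.
; Overlap by BP_SparkCharacter_Player passes its PlayerStart to BP_SparkGameInstance through SetCheckpoint.
; A DoOnce gates the trigger and resets immediately unless TriggerOnce is set, though any first overlapping actor consumes it before the player cast.
; UpdateCheckpoint is empty, and disconnected nodes hold unfinished logic for replacing the PlayerStart.
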(event `self.ReceiveBeginPlay`)

(event `self.Trigger.OnComponentBeginOverlap`
  (params (OverlappedComponent :type "PrimitiveComponent Object Reference") (OtherActor :type "Actor Object Reference") (OtherComp :type "PrimitiveComponent Object Reference") (OtherBodyIndex :type Integer) (bFromSweep :type Boolean) (SweepResult :type "HitResult Structure (by ref)"))
  (`/Engine/EditorBlueprintResources/StandardMacros.DoOnce` false :!label _label
    (:`Completed`
      (cast `/Game/Gameplay/Characters/Player/BP_SparkCharacter_Player` OtherActor)
      (bind _asbp_spark_game_instance (cast `/Game/Gameplay/Modes/BP_SparkGameInstance` (`GameplayStatics.GetGameInstance`)))
      (`/Game/Gameplay/Modes/BP_SparkGameInstance.Set Checkpoint` _asbp_spark_game_instance (`self.player_start`))
      (if (not (`self.bTriggerOnce`))
        (`self.ResetCheckpoint`)))))

(event `ResetCheckpoint`
  (goto _label :!via `Reset`))

(event `Update Checkpoint`)

(fn `UserConstructionScript`)