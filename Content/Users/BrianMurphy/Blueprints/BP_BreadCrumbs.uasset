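; BP_BreadCrumbs is an actor that places instances of a chosen actor class along a spline as breadcrumbs.
; SpawnBreadcrumbs gets transforms from TransformsAlongSpline, spawns ActorToInstance at each, and sets the matching SpawnedActors index, though no spawned actor is shown wired into that set.
; ClearBreadcrumbs destroys every actor in SpawnedActors without emptying the array.
; BeginPlay and the construction script are empty, and nothing here calls either event.
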(event `SpawnBreadcrumbs`
  (bind _outtransforms (`/Game/Users/BrianMurphy/Blueprints/BPFL_SplineFunctions.Transforms Along Spline` (`self.Spline`)))
  (for (_array_element _array_index) _outtransforms
    (`|SpawnActorFromClass` (`self.Actor to Instance`) _array_element "Undefined" "OverrideRootScale" null null)
    (`KismetArrayLibrary.Array_Set` (`self.SpawnedActors`) _array_index)))

(event `ClearBreadcrumbs`
  (for _array_element (`self.SpawnedActors`)
    (`self.K2_DestroyActor` _array_element)))

(event `self.ReceiveBeginPlay`)

(fn `UserConstructionScript`)