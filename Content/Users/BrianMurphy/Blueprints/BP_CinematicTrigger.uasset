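; One-shot cinematic trigger that plays a level sequence when its box is first overlapped, then starts the boss fight.
; If the overlapping actor is the Stormwrak player character, it disables that player's input and stops their charging.
; A delay computed from the sequence's frame duration and rate, rather than a finish callback, times the ending.
; SequenceEnded then tells the first BP_Boss found to start shooting and restores the stored player's input.
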(event `PlaySequence`
  (bind (_outactor _returnvalue) (`LevelSequencePlayer.CreateLevelSequencePlayer` (`self.Seq`)))
  (`MovieSceneSequencePlayer.Play` _returnvalue)
  (bind _returnvalue_numerator (`KismetMathLibrary.BreakFrameRate` (`MovieSceneSequencePlayer.GetFrameRate` _returnvalue)))
  (`KismetSystemLibrary.Delay` (`KismetMathLibrary.Conv_IntToDouble` (/ (`MovieSceneSequencePlayer.GetFrameDuration` _returnvalue) _returnvalue_numerator)))
  (`self.Sequence Ended`))

(event `self.Box.OnComponentBeginOverlap`
  (params (OverlappedComponent :type "PrimitiveComponent Object Reference") (OtherActor :type "Actor Object Reference") (OtherComp :type "PrimitiveComponent Object Reference") (OtherBodyIndex :type Integer) (bFromSweep :type Boolean) (SweepResult :type "HitResult Structure (by ref)"))
  (`/Engine/EditorBlueprintResources/StandardMacros.DoOnce` false
    (:`Completed`
      (bind _asbp_spark_character_player_stormwrak (cast `/Game/Users/BrianMurphy/Blueprints/BP_SparkCharacter_Player_Stormwrak` OtherActor)
        (:`then`
          (bind _output_get (set `self.As BP Spark Character Player Stormwrak` _asbp_spark_character_player_stormwrak))
          (`self.DisableInput` _asbp_spark_character_player_stormwrak (`GameplayStatics.GetPlayerController` 0))
          (`/Game/Gameplay/Characters/Player/BP_SparkCharacter_Player.StopCharging` _output_get))
        (:`CastFailed`
          _))
      (`self.PlaySequence`))))

(event `Sequence Ended`
  (bind _as_bp_spark_character_player_stormwrak (`self.As BP Spark Character Player Stormwrak`))
  (`|ExecutionSequence`
    (:`then_0`
      (bind _outactors (`GameplayStatics.GetAllActorsOfClass` "/Game/Users/BrianMurphy/Blueprints/BP_Boss.BP_Boss_C"))
      (`/Game/Users/BrianMurphy/Blueprints/BP_Boss.StartShooting` (`|GetArrayItem` _outactors)))
    (:`then_1`
      (`/Engine/EditorBlueprintResources/StandardMacros.IsValid` _as_bp_spark_character_player_stormwrak
        (:`Is Valid`
          (`self.EnableInput` _as_bp_spark_character_player_stormwrak (`GameplayStatics.GetPlayerController` 0)))))))

(fn `UserConstructionScript`)