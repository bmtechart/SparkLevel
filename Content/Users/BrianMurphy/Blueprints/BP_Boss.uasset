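; BP_Boss is a boss that bombards the Stormwrak Spark player with bombs and leaves a return portal when it dies.
; ShootAtTarget spawns a fused BP_Bomb above the target, while StartShooting and StopShooting run and pause a looping timer.
; Damage outside its immunities goes through DamageCharacter, leading to Death, which destroys the boss, or an empty DamageBoss hook.
; IsTargetViable traces upward for overhead cover but is not called here.
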(event `Shoot_FX`
  (bind _cannonballspawn (`self.CannonBallSpawn`))
  ;[1 1 1] Show effects on boss
  (`GameplayStatics.PlaySound2D` "/Game/Users/BrianMurphy/Audio/explosion_far_distant_02.explosion_far_distant_02" 1.0 1.0 0.0 null null)
  (`GameplayStatics.SpawnEmitterAtLocation` "/Game/Environments/Pirates/ParticleFX/P_FX_Cannon_Fire.P_FX_Cannon_Fire" (`SceneComponent.K2_GetComponentLocation` _cannonballspawn) (`SceneComponent.K2_GetComponentRotation` _cannonballspawn)))

(event `SetTarget`
  (params (TargetActor :type "Actor Object Reference"))
  (set `self.target` TargetActor))

(event `GetTarget`
  ;[1 1 1] Get reference to player
  (bind _outactors (`GameplayStatics.GetAllActorsOfClass` "/Game/Users/BrianMurphy/Blueprints/BP_SparkCharacter_Player_Stormwrak.BP_SparkCharacter_Player_Stormwrak_C"))
  (set `self.Spark` (`|GetArrayItem` _outactors)))

(event `StopShooting`
  ;[1 1 1] Enable/Disable Shooting
  (if (`KismetSystemLibrary.K2_IsValidTimerHandle` (`self.ShootEventHandle`))
    (`KismetSystemLibrary.K2_PauseTimerHandle` (`self.ShootEventHandle`))))

(event `ShootAtTarget`
  (bind (_returnvalue_x _returnvalue_y _returnvalue_z) (`KismetMathLibrary.BreakVector` (`self.K2_GetActorLocation` (`self.target`))))
  ;[1 1 1] Shoot cannonball at player
  (`/Engine/EditorBlueprintResources/StandardMacros.IsValid` (`self.target`)
    (:`Is Valid`
      (bind _returnvalue (`|SpawnActorFromClass` "/Game/Users/BrianMurphy/Blueprints/BP_Bomb.BP_Bomb_C" (`KismetMathLibrary.MakeTransform` (`KismetMathLibrary.MakeVector` _returnvalue_x _returnvalue_y (+ _returnvalue_z (`self.Spawn Z Offset`)))) "Undefined" "OverrideRootScale" null null))
      (`KismetSystemLibrary.PrintString` "spawned bomb")
      (`/Game/Users/BrianMurphy/Blueprints/BP_Bomb.StartFuse` _returnvalue))
    (:`Is Not Valid`
      (`KismetSystemLibrary.PrintString` "Shoot At Event Error: No viable target to shoot at!"))))

(event `StartShooting`
  ;[1 1 1] Enable/Disable Shooting
  (`/Engine/EditorBlueprintResources/StandardMacros.IsValid` (`self.target`)
    (:`Is Valid`
      _)
    (:`Is Not Valid`
      (`self.GetTarget`)))
  (if (`KismetSystemLibrary.K2_IsValidTimerHandle` (`self.ShootEventHandle`))
    (`KismetSystemLibrary.K2_UnPauseTimerHandle` (`self.ShootEventHandle`))
    (else
      (bind _returnvalue (`KismetSystemLibrary.K2_SetTimerDelegate` (`|CreateDelegate` :!event `ShootAtTarget`) 2.0 true))
      (set `self.ShootEventHandle` _returnvalue))))

(event `self.ReceiveAnyDamage`
  (params (Damage :type "Float (single-precision)") (DamageType :type "DamageType Object Reference") (InstigatedBy :type "Controller Object Reference") (DamageCauser :type "Actor Object Reference"))
  ;[1 1 1] Damag
  (if (not (`BlueprintSetLibrary.Set_Contains` (`self.DamageImmunities`) (`GameplayStatics.GetObjectClass` DamageType)))
    (bind _isdead (`self.DamageCharacter` 1.0))
    (if _isdead
      (`self.Death`)
      (else
        (`self.DamageBoss`)
        (`KismetSystemLibrary.PrintString` "boss damaged")))))

(event `self.ReceiveBeginPlay`)

(event `Death`
  (bind _outhit (`KismetSystemLibrary.LineTraceSingle` (`self.K2_GetActorLocation` self) (0.0 0.0 0.0) "TraceTypeQuery1"))
  (`|SpawnActorFromClass` "/Game/Gameplay/Objects/BP_ReturnPortal.BP_ReturnPortal_C" (`KismetMathLibrary.MakeTransform` (`.Location` (`GameplayStatics.BreakHitResult` _outhit))) "Undefined" "OverrideRootScale" null null)
  (`self.K2_DestroyActor`))

(event `DamageBoss`)

(event `BossAttack_Bombard`)

(fn `IsTargetViable`
  (returns (ReturnValue :type Boolean))
  (bind _target (`self.target`))
  (bind (_returnvalue_x _returnvalue_y _returnvalue_z) (`KismetMathLibrary.BreakVector` (`self.K2_GetActorLocation` _target)))
  (bind (_outhit _returnvalue) (`KismetSystemLibrary.LineTraceSingle` (`self.K2_GetActorLocation` _target) (`KismetMathLibrary.MakeVector` _returnvalue_x _returnvalue_y (+ _returnvalue_z 10000.0)) "TraceTypeQuery1"))
  (return (not _returnvalue)))

(fn `UserConstructionScript`)