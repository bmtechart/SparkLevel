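; BP_Bomb is an explosive actor that lights its fuse when it takes point damage.
; StartFuse attaches a fuse effect and sets the bomb's sphere to ignore the Visibility channel, then waits out a configurable delay.
; It then deals full radial damage using the flame breath damage type, draws a debug sphere of the blast radius, plays an explosion sound and destroys itself.
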(event `self.ReceiveBeginPlay`)

(event `self.ReceivePointDamage`
  (params (Damage :type "Float (single-precision)") (DamageType :type "DamageType Object Reference") (HitLocation :type "Vector Structure") (HitNormal :type "Vector Structure") (HitComponent :type "PrimitiveComponent Object Reference") (BoneName :type Name) (ShotFromDirection :type "Vector Structure") (InstigatedBy :type "Controller Object Reference") (DamageCauser :type "Actor Object Reference") (HitInfo :type "HitResult Structure (by ref)"))
  (`self.StartFuse\\`))

(event `StartFuse\\`
  (bind _fusefxlocation (`self.FuseFXLocation`))
  (`NiagaraFunctionLibrary.SpawnSystemAttached` "/Game/Users/BrianMurphy/FX/FX_BombFuse_System.FX_BombFuse_System" _fusefxlocation "None" (`SceneComponent.K2_GetComponentLocation` _fusefxlocation) (`SceneComponent.K2_GetComponentRotation` _fusefxlocation) "SnapToTarget" false true "None" false)
  (`PrimitiveComponent.SetCollisionResponseToChannel` (`self.Sphere1`) "ECC_Visibility" "ECR_Ignore")
  (`KismetSystemLibrary.Delay` (`self.FuseDelay`))
  (`GameplayStatics.ApplyRadialDamage` :`BaseDamage` (`KismetMathLibrary.Conv_IntToDouble` (`self.Damage`)) :`Origin` (`SceneComponent.K2_GetComponentLocation` (`self.Sphere1`)) :`DamageRadius` (`self.ExplosionRadius`) :`DamageTypeClass` "/Game/Gameplay/Logic/DamageTypes/DT_FlameBreath.DT_FlameBreath_C" :`DamageCauser` null :`InstigatedByController` null :`bDoFullDamage` true)
  (`KismetSystemLibrary.DrawDebugSphere` (`SceneComponent.K2_GetComponentLocation` (`self.Sphere1`)) (`self.ExplosionRadius`) 12 (struct :`R` 1.0 :`G` 1.0 :`B` 1.0 :`A` 1.0) 2.0)
  (`GameplayStatics.PlaySoundAtLocation` "/Game/Objects/Chest/Sound/S_ChestExplosion.S_ChestExplosion" (`SceneComponent.K2_GetComponentLocation` (`self.Sphere1`)) (struct) 0.35 1.0 0.0 null null null)
  (`self.K2_DestroyActor`))

(fn `UserConstructionScript`)