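; BP_Bonfire is a bonfire actor that lights up when hit by flame breath damage.
; On BeginPlay it hides its particle system by scaling it to zero.
; AnyDamage of type DT_FlameBreath scales the particles up and plays GoOutTimeline, though no logic is shown on that timeline's outputs.
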(event `self.ReceiveBeginPlay`
  (`parent.ReceiveBeginPlay`)
  (`SceneComponent.SetWorldScale3D` (`self.ParticleSystem`) (0.0 0.0 0.0)))

(event `self.ReceiveAnyDamage`
  (params (Damage :type "Float (single-precision)") (DamageType :type "DamageType Object Reference") (InstigatedBy :type "Controller Object Reference") (DamageCauser :type "Actor Object Reference"))
  (if (== DamageType "/Game/Gameplay/Logic/DamageTypes/DT_FlameBreath.DT_FlameBreath")
    (`SceneComponent.SetWorldScale3D` (`self.ParticleSystem`) (2.0 2.0 2.0))
    (`Timeline|GoOutTimeline`)))

(fn `UserConstructionScript`
  (`parent.UserConstructionScript`))