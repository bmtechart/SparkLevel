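; Boss attack Blueprint that periodically drops bombs on the Spark player character.
; BeginPlay starts a pausable looping timer, apparently driving ShootAtTarget, which finds the player and traces upward from them to confirm open sky.
; If clear, it plays a distant explosion sound, then after a delay spawns a BP_Bomb above the player's current position and lights its fuse.
; Older cannonball spline-arc and look-at aiming logic remains but is disconnected.
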(event `StopShooting`
  ;[1 1 1] ShootingBehaviour
  (if (`KismetSystemLibrary.K2_IsValidTimerHandle` (`self.ShootEventHandle`))
    (`KismetSystemLibrary.K2_PauseTimerHandle` (`self.ShootEventHandle`))))

(event `StartShooting`
  ;[1 1 1] ShootingBehaviour
  (if (`KismetSystemLibrary.K2_IsValidTimerHandle` (`self.ShootEventHandle`))
    (`KismetSystemLibrary.K2_UnPauseTimerHandle` (`self.ShootEventHandle`))
    (else
      (bind _returnvalue (`KismetSystemLibrary.K2_SetTimerDelegate` (`|CreateDelegate` :!event `ShootAtTarget`) 2.0 true))
      (set `self.ShootEventHandle` _returnvalue))))

(event `CheckTargetViability`
  (`/Engine/EditorBlueprintResources/StandardMacros.IsValid` (`self.Spark`)))

(event `self.ReceiveBeginPlay`
  (`self.StartShooting`))

(event `ShootAtTarget`
  (bind (_returnvalue_x _returnvalue_y _returnvalue_z) (`KismetMathLibrary.BreakVector` (`self.K2_GetActorLocation` (`self.Spark`))))
  ;[1 1 1] Comment
  (`/Engine/EditorBlueprintResources/StandardMacros.IsValid` (`self.Spark`)
    (:`Is Valid`
      _)
    (:`Is Not Valid`
      (`self.GetTarget`)))
  (if (`self.IsTargetViable`)
    (`GameplayStatics.PlaySound2D` "/Game/Users/BrianMurphy/Audio/explosion_far_distant_02.explosion_far_distant_02" 1.0 1.0 0.0 null null)
    (`KismetSystemLibrary.Delay` 1.5)
    (bind _returnvalue (`|SpawnActorFromClass` "/Game/Users/BrianMurphy/Blueprints/BP_Bomb.BP_Bomb_C" (`KismetMathLibrary.MakeTransform` (`KismetMathLibrary.MakeVector` _returnvalue_x _returnvalue_y (+ _returnvalue_z 500.0))) "Undefined" "OverrideRootScale" null null))
    (`/Game/Users/BrianMurphy/Blueprints/BP_Bomb.StartFuse\\` _returnvalue)))

(event `GetTarget`
  ;[1 1 1] Track target
  ;;[1 1 1] Get reference to player
  (bind _outactors (`GameplayStatics.GetAllActorsOfClass` "/Game/Users/BrianMurphy/Blueprints/BP_SparkCharacter_Player_Stormwrak.BP_SparkCharacter_Player_Stormwrak_C"))
  (set `self.Spark` (`|GetArrayItem` _outactors)))

(event `self.ReceiveTick`
  (params (DeltaSeconds :type "Float (single-precision)"))
  ;[0 1 0.25 1 361] Deprecated
  (`|ExecutionSequence`))

(event `BuildCannonBallPath`
  (bind _returnvalue (`SceneComponent.K2_GetComponentLocation` (`self.CannonBallSpawn`)))
  (bind _returnvalue_2 (`self.K2_GetActorLocation` (`self.Spark`)))
  (bind (_returnvalue_x _returnvalue_y _returnvalue_z) (`KismetMathLibrary.BreakVector` (/ (+ _returnvalue _returnvalue_2) 2.0)))
  ;[0 1 0.25 1 361] Deprecated
  (`|ExecutionSequence`
    (:`then_0`
      (`SplineComponent.ClearSplinePoints` (`self.CannonPath`) true))
    (:`then_1`
      ;;[1 1 1] Debug Cannonball path
      (`SplineComponent.SetSplinePoints` (`self.CannonPath`) (`|MakeArray` _returnvalue (`KismetMathLibrary.MakeVector` _returnvalue_x _returnvalue_y (+ _returnvalue_z 500.0)) _returnvalue_2) "World" true))))

(fn `IsTargetViable`
  (returns (ReturnValue :type Boolean))
  (bind _spark (`self.Spark`))
  (bind (_returnvalue_x _returnvalue_y _returnvalue_z) (`KismetMathLibrary.BreakVector` (`self.K2_GetActorLocation` _spark)))
  (bind (_outhit _returnvalue) (`KismetSystemLibrary.LineTraceSingle` (`self.K2_GetActorLocation` _spark) (`KismetMathLibrary.MakeVector` _returnvalue_x _returnvalue_y (+ _returnvalue_z 10000.0)) "TraceTypeQuery1"))
  (return (not _returnvalue)))

(fn `UserConstructionScript`)