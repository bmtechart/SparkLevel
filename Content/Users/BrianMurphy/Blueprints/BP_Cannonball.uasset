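; BP_Cannonball is a projectile actor that flies along a spline path and explodes at the end.
; BeginPlay builds the world-space spline from the SplinePoints array.
; Tick advances a distance by TravelRate and delta time, moving the mesh there with a sweep.
; When that spline location nears the third point, PathEnded spawns explosion FX and sound at the mesh, then destroys the actor.
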(event `self.ReceiveBeginPlay`
  (`SplineComponent.SetSplinePoints` (`self.Spline`) (`self.SplinePoints`) "World" true))

(event `self.ReceiveTick`
  (params (DeltaSeconds :type "Float (single-precision)"))
  (bind _output_get (set `self.Spline Position` (+ (* DeltaSeconds (`self.TravelRate`)) (`self.Spline Position`))))
  (bind _returnvalue (`SplineComponent.GetLocationAtDistanceAlongSpline` (`self.Spline`) _output_get "World"))
  (`SceneComponent.K2_SetWorldLocation` (`self.StaticMesh`) _returnvalue true false)
  (if (== _returnvalue (`|GetArrayItem` (`self.SplinePoints`) 2) :`ErrorTolerance` 0.1)
    (`self.PathEnded`)))

(event `PathEnded`
  (bind _returnvalue (`SceneComponent.K2_GetComponentLocation` (`self.StaticMesh`)))
  (`NiagaraFunctionLibrary.SpawnSystemAtLocation` "/Game/Users/BrianMurphy/FX/FX_CannonExplosion_System.FX_CannonExplosion_System" _returnvalue)
  (`GameplayStatics.PlaySoundAtLocation` "/Game/Users/BrianMurphy/Audio/explosion_large_08.explosion_large_08" _returnvalue (struct) 0.2 1.0 0.0 null null null)
  (`self.K2_DestroyActor`))

(fn `UserConstructionScript`)