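; Spline track actor that moves a child actor along its spline, optionally starting on BeginPlay.
; A timeline track supplies the spline input key, and each update moves the child to that world location with sweep.
; StartTrack, PauseTrack and ReverseTrack control the timeline, with reverse always playing from the end.
; When Loop is set, the finished timeline flips direction to ping-pong the child back and forth.
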(event `self.ReceiveBeginPlay`
  (if (`self.AutoStart`)
    (`self.StartTrack`)))

(event `StartTrack`
  (bind (_direction _newtrack_0) (`Timeline|Timeline_0` :!label _label)
    (:`Update`
      (`self.K2_SetActorLocation` (`self.ChildActor`) (`SplineComponent.GetLocationAtSplineInputKey` (`self.Spline`) _newtrack_0 "World") true false))
    (:`Finished`
      (if (`self.Loop`)
        (switch `ETimelineDirection` _direction
          (:`Forward`
            (`self.ReverseTrack`))
          (:`Backward`
            (`self.StartTrack`)))))))

(event `PauseTrack`
  (goto _label :!via `Stop`))

(event `ReverseTrack`
  (goto _label :!via `ReverseFromEnd`))

(fn `UserConstructionScript`)