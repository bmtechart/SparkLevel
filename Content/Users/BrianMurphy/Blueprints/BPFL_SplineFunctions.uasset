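; Blueprint function library with a spline helper that returns an array of evenly spaced transforms between normalized start and end positions on a spline.
; The instance count comes from the segment length divided by Density, so Density acts as spacing, with optional clamping to a maximum.
; A loop lerps distance across the segment and samples transforms in the chosen coordinate space, optionally with spline scale.
; It spawns nothing, and ActorToInstance is unused.
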(fn `Transforms Along Spline`
  (params (Spline :type "SplineComponent Object Reference") (ActorToInstance :type "Actor Class Reference") (Density :type "Float (double-precision)") (StartPosition :type "Float (double-precision)") (EndPosition :type "Float (double-precision)") (`ClampInstances?` :type Boolean) (MaxInstances :type Integer) (`UseSplineScale?` :type Boolean) (CoordinateSpace :type "ESplineCoordinateSpace Enum" :default "Local"))
  (returns (OutTransforms :type "Array of Transform Structure"))
  (locals (NumInstances :type Integer) (OutTransformArray :type "Array of Transform Structure"))
  (bind _returnvalue (`SplineComponent.GetSplineLength` (`local.Spline`)))
  (bind _returnvalue_2 (`SplineComponent.GetSplineLength` (`local.Spline`)))
  (bind _returnvalue_3 (`KismetMathLibrary.Round` (/ (- (- _returnvalue_2 (* _returnvalue_2 (`local.StartPosition`))) (* _returnvalue_2 (- 1.0 (`local.EndPosition`)))) (`local.Density`))))
  (`|ExecutionSequence`
    (:`then_0`
      ;[1 1 1] Determine number of instances to spawn
      (set `local.NumInstances` (select `bool` (`local.ClampInstances?`) :`false` _returnvalue_3 :`true` (`KismetMathLibrary.Clamp` _returnvalue_3 1 (`local.MaxInstances`)))))
    (:`then_1`
      (for _index (range (+ (`local.NumInstances`) 1))
        (`KismetArrayLibrary.Array_Add` (`local.OutTransformArray`) (`SplineComponent.GetTransformAtDistanceAlongSpline` (`local.Spline`) (`KismetMathLibrary.Lerp` (* _returnvalue (`local.StartPosition`)) (* _returnvalue (`local.EndPosition`)) (/ (`KismetMathLibrary.Conv_IntToDouble` _index) (`KismetMathLibrary.Conv_IntToDouble` (`local.NumInstances`)))) CoordinateSpace (`local.UseSplineScale?`)))))
    (:`then_2`
      (return (`local.OutTransformArray`)))))