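; BP_Rain is a rain actor that keeps itself positioned above a follow target.
; Every Tick, if the target is valid, it teleports its root to the target's location, raised by ZOffSet.
; SetFollowTarget ignores its NewFollowTarget input and instead stores the first BP_SparkCharacter_Player found in the world.
; Nothing in this graph calls SetFollowTarget, and BeginPlay is empty.
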(event `self.ReceiveTick`
  (params (DeltaSeconds :type "Float (single-precision)"))
  (bind (_returnvalue_x _returnvalue_y _returnvalue_z) (`KismetMathLibrary.BreakVector` (`self.K2_GetActorLocation` (`self.FollowTarget`))))
  (`/Engine/EditorBlueprintResources/StandardMacros.IsValid` (`self.FollowTarget`)
    (:`Is Valid`
      (`SceneComponent.K2_SetWorldLocation` (`self.DefaultSceneRoot`) (`KismetMathLibrary.MakeVector` _returnvalue_x _returnvalue_y (+ _returnvalue_z (`self.ZOffSet`))) false true))))

(event `SetFollowTarget`
  (params (NewFollowTarget :type "Actor Object Reference"))
  (bind _outactors (`GameplayStatics.GetAllActorsOfClass` "/Game/Gameplay/Characters/Player/BP_SparkCharacter_Player.BP_SparkCharacter_Player_C"))
  (set `self.FollowTarget` (`|GetArrayItem` _outactors)))

(fn `UserConstructionScript`)