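; BP_SplineInstancer spawns copies of an InstanceActor class at even intervals along TargetSpline.
; SpawnActors destroys the previous batch, then derives the count from spline length divided by InstanceDensity, clamped to MaxInstances, so density acts as spacing.
; Each actor follows the spline's world location and rotation, with an added 90-degree local turn, and is tracked in SpawnedActors.
; ClearActors destroys the tracked actors; BeginPlay and the construction script are empty.
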(event `Clear Actors`
  (for _array_element (`self.SpawnedActors`)
    (`self.K2_DestroyActor` _array_element))
  (`KismetArrayLibrary.Array_Clear` (`self.SpawnedActors`)))

(event `SpawnActors`
  (bind _targetspline (`self.TargetSpline`))
  (if (> (`KismetArrayLibrary.Array_Length` (`self.SpawnedActors`)) 0)
    (for _array_element (`self.SpawnedActors`)
      (`self.K2_DestroyActor` _array_element))
    (`KismetArrayLibrary.Array_Clear` (`self.SpawnedActors`)))
  (bind _output_get (set `self.NumInstances` (`KismetMathLibrary.Conv_IntToDouble` (`KismetMathLibrary.Clamp` (`KismetMathLibrary.Round` (/ (`SplineComponent.GetSplineLength` (`self.TargetSpline`)) (`self.InstanceDensity`))) 1 (`self.MaxInstances`)))))
  (for _index (range (+ (`KismetMathLibrary.FTrunc` _output_get) 1))
    (bind _returnvalue (* (`SplineComponent.GetSplineLength` (`self.TargetSpline`)) (/ (`KismetMathLibrary.Conv_IntToDouble` _index) (`self.NumInstances`))))
    (bind _returnvalue_2 (`|SpawnActorFromClass` (`self.InstanceActor`) (`KismetMathLibrary.MakeTransform` (`SplineComponent.GetLocationAtDistanceAlongSpline` _targetspline _returnvalue "World") (`SplineComponent.GetRotationAtDistanceAlongSpline` _targetspline _returnvalue "World")) "Undefined" "OverrideRootScale" null null))
    (`self.K2_AddActorLocalRotation` _returnvalue_2 (struct :`Yaw` 90.0) false false)
    (`KismetArrayLibrary.Array_AddUnique` (`self.SpawnedActors`) _returnvalue_2)))

(event `self.ReceiveBeginPlay`)

(fn `UserConstructionScript`)