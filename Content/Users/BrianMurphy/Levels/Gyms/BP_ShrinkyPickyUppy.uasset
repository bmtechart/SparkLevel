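; BP_ShrinkyPickyUppy is a gym-level actor that smoothly shrinks whatever actor begins overlapping its Sphere component.
; The overlap stores the actor and its initial scale, then starts a fast looping timer that interpolates its scale toward TargetScale and pauses on arrival.
; Each overlap replaces the stored actor and timer handle without clearing the previous timer, and the saved initial scale is never read here.
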(event `self.Sphere.OnComponentBeginOverlap`
  (params (OverlappedComponent :type "PrimitiveComponent Object Reference") (OtherActor :type "Actor Object Reference") (OtherComp :type "PrimitiveComponent Object Reference") (OtherBodyIndex :type Integer) (bFromSweep :type Boolean) (SweepResult :type "HitResult Structure (by ref)"))
  (bind _output_get (set `self.ActorToShrink` OtherActor))
  (set `self.InitScale` (`self.GetActorScale3D` _output_get))
  (bind _returnvalue (`KismetSystemLibrary.K2_SetTimerDelegate` (delegate `ShrinkTarget`) 0.001 true))
  (set `self.ScaleEventTimer` _returnvalue))

(event `ShrinkTarget`
  (bind _actortoshrink (`self.ActorToShrink`))
  (`/Engine/EditorBlueprintResources/StandardMacros.IsValid` _actortoshrink
    (:`Is Valid`
      (`self.SetActorScale3D` _actortoshrink (`KismetMathLibrary.VInterpTo` (`self.GetActorScale3D` (`self.ActorToShrink`)) (`self.TargetScale`) (`GameplayStatics.GetWorldDeltaSeconds`) (`self.ShrinkSpeed`)))
      ;[1 1 1] Stop Shrinking Once We are Shrunk
      (if (== (`self.GetActorScale3D` (`self.ActorToShrink`)) (`self.TargetScale`))
        (`KismetSystemLibrary.K2_PauseTimerHandle` (`self.ScaleEventTimer`))))))

(fn `UserConstructionScript`)